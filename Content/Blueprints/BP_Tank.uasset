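; BP_Tank is a drivable tank with a team colour, an HP bar widget and an explosion effect when destroyed.
; BeginPlay hands barrel and turret to TankAiming and tracks to TankMovement, links the HP bar to itself, and paints body, turret and barrel blue or red by TeamFlag.
; Input orbits the spring-arm camera with clamped pitch, fires through TankAiming, and drives via TankMovement or per-track throttles.
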(event EventBeginPlay
  (Class|TankAimingComponent|Initalize (Variables|Default|GetTankAiming) (Variables|Default|GetTankBarrel) (Variables|Default|GetTankTurret))
  (Class|TankMovementComponent|Initalize (Variables|Default|GetTankMovement) (Variables|Default|GetLeftTrack) (Variables|Default|GetRightTrack))
  (bind _ashp_bar (Utilities|Casting|CastToHpBar (UserInterface|GetUserWidgetObject (Variables|Default|GetHpBarWidget))))
  (Variables|/Game/Blueprints/UI/HpBar.HpBar_C|SetTank _ashp_bar self)
  (Rendering|SetVisibility (Variables|Default|GetHpBarWidget) true true)
  (if (Variables|Default|GetTeamFlag)
    (Variables|Default|Setmaterial "/Game/Assests/M_Blue.M_Blue")
    (else
      (Variables|Default|Setmaterial "/Game/Assests/M_Red.M_Red")))
  (Rendering|Material|SetMaterial (Variables|Default|GetTankBody) 0 (Variables|Default|Getmaterial))
  (Rendering|Material|SetMaterial (Variables|Default|GetTankTurret) 0 (Variables|Default|Getmaterial))
  (Rendering|Material|SetMaterial (Variables|Default|GetTankBarrel) 0 (Variables|Default|Getmaterial)))

(event Collision|EventActorBeginOverlap
  (params (OtherActor :type Actor%20Object%20Reference)))

(event EventTick
  (params (DeltaSeconds :type Float%20%28single-precision%29)))

(event EventDestroyed
  (Effects|SpawnEmitteratLocation "/Game/Blueprints/Projectile/P_TankExplosion.P_TankExplosion" (Transformation|GetActorLocation)))

(event Input|ActionEvents|InputActionFire
  (params (Key :type Key%20Structure))
  (:Pressed
    (Class|TankAimingComponent|Fire (Variables|Default|GetTankAiming))))

(event Input|AxisEvents|InputAxisLookH
  (params (AxisValue :type Float%20%28single-precision%29))
  (Transformation|AddRelativeRotation (Variables|Default|GetScene) (Math|Rotator|MakeRotator 0.0 0.0 AxisValue) false false))

(event Input|AxisEvents|InputAxisLeftTrackThrottle
  (params (AxisValue :type Float%20%28single-precision%29))
  (Class|TankTrack|SetThrottle (Variables|Default|GetLeftTrack) AxisValue))

(event Input|AxisEvents|InputAxisRightTrackThrottle
  (params (AxisValue :type Float%20%28single-precision%29))
  (Class|TankTrack|SetThrottle (Variables|Default|GetRightTrack) AxisValue))

(event Input|AxisEvents|InputAxisLookV
  (params (AxisValue :type Float%20%28single-precision%29))
  (bind _springarm (Variables|Default|GetSpringArm))
  (bind _relativerotation (Variables|/Script/Engine.SceneComponent|GetRelativeRotation _springarm))
  (Transformation|SetRelativeRotation (Variables|Default|GetSpringArm) (Math|Rotator|MakeRotator (.roll _relativerotation) (Math|Float|Clamp(Float) (+ AxisValue (.pitch _relativerotation)) -4e+01 5.0) (.yaw _relativerotation)) false false))

(event Input|AxisEvents|InputAxisMoveForward
  (params (AxisValue :type Float%20%28single-precision%29))
  (Class|TankMovementComponent|MoveForward (Variables|Default|GetTankMovement) AxisValue))

(event Input|AxisEvents|InputAxisMoveRight
  (params (AxisValue :type Float%20%28single-precision%29))
  (Class|TankMovementComponent|MoveRight (Variables|Default|GetTankMovement) AxisValue))

(fn ConstructionScript)